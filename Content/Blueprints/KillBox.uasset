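; KillBox is a trigger volume that destroys whatever enters its box and respawns the player.
; When a BP_PlayerCharacter overlaps, it is destroyed and a fresh one spawns at the first PlayerStart found in the level.
; The new character has IsDragQueen cleared, is possessed by player controller 0, and any camera fade is stopped.
; Any other overlapping actor is simply destroyed.
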(event `self.ReceiveActorBeginOverlap`
  (params (OtherActor :type "Actor Object Reference")))

(event `self.Box.OnComponentBeginOverlap`
  (params (OverlappedComponent :type "PrimitiveComponent Object Reference") (OtherActor :type "Actor Object Reference") (OtherComp :type "PrimitiveComponent Object Reference") (OtherBodyIndex :type Integer) (bFromSweep :type Boolean) (SweepResult :type "HitResult Structure (by ref)"))
  (bind _asbp_player_character (cast `/Game/Character/BP_PlayerCharacter` OtherActor)
    (:`then`
      (`self.K2_DestroyActor` _asbp_player_character)
      (bind _outactors (`GameplayStatics.GetAllActorsOfClass` "/Script/Engine.PlayerStart"))
      (bind _returnvalue (`|SpawnActorFromClass` "/Game/Character/BP_PlayerCharacter.BP_PlayerCharacter_C" (`self.GetTransform` (`|GetArrayItem` _outactors)) "Undefined" "OverrideRootScale" null null))
      (set `/Game/Character/BP_PlayerCharacter.isDragQueen` false _returnvalue)
      (`Controller.Possess` (`GameplayStatics.GetPlayerController` 0) _returnvalue)
      (`PlayerCameraManager.StopCameraFade` (`GameplayStatics.GetPlayerCameraManager` 0)))
    (:`CastFailed`
      (`self.K2_DestroyActor` OtherActor))))

(fn `UserConstructionScript`)