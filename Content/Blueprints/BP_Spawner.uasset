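; BP_Spawner is an actor that continuously spawns BP_Tree actors while the game runs.
; On BeginPlay it reads TreeRate from MyGameMode, then SpawnTree calls itself again after a random delay capped by that rate.
; GetTreeSpawn places each tree at the Center component's transform, offset randomly along world Y within a wide band.
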(event `self.ReceiveBeginPlay`
  (bind _asmy_game_mode (cast `/Game/Gameplay/MyGameMode` (`GameplayStatics.GetGameMode`)))
  (set `self.TreeRate` (`/Game/Gameplay/MyGameMode.TreeRate` _asmy_game_mode))
  (`self.SpawnTree`))

(event `SpawnTree`
  (bind _returnvalue1 (`self.GetTreeSpawn`))
  (`|SpawnActorFromClass` "/Game/Blueprints/BP_Tree.BP_Tree_C" _returnvalue1 "Undefined" "OverrideRootScale" null null)
  (`KismetSystemLibrary.Delay` (`KismetMathLibrary.RandomFloatInRange` 0.01 (`self.TreeRate`)))
  (`self.SpawnTree`))

(fn `GetTreeSpawn`
  (returns (ReturnValue1 :type "Transform Structure"))
  (return (`KismetMathLibrary.MakeTransform` (`KismetMathLibrary.MakeVector` (.x (.location (`SceneComponent.K2_GetComponentToWorld` (`self.Center`)))) (+ (.y (.location (`SceneComponent.K2_GetComponentToWorld` (`self.Center`)))) (`KismetMathLibrary.RandomFloatInRange` -20000.0 20000.0)) (.z (.location (`SceneComponent.K2_GetComponentToWorld` (`self.Center`))))) (.rotation (`SceneComponent.K2_GetComponentToWorld` (`self.Center`))) (.scale (`SceneComponent.K2_GetComponentToWorld` (`self.Center`))))))

(fn `UserConstructionScript`)