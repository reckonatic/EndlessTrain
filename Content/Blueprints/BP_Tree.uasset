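; BP_Tree is a tree actor that scrolls steadily along the world X axis, likely as moving scenery.
; On BeginPlay, RandomMesh adds one of ten static mesh components, picked at random, to vary its appearance.
; The construction script reads Speed from MyGameMode, and Tick offsets the X location by Speed scaled by delta time, without sweeping.
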(event `self.ReceiveBeginPlay`
  (`self.RandomMesh`))

(event `self.ReceiveTick`
  (params (DeltaSeconds :type "Float (single-precision)"))
  (`self.K2_SetActorLocation` (`KismetMathLibrary.MakeVector` (+ (.x (`self.K2_GetActorLocation`)) (* DeltaSeconds (`self.speed`))) (.y (`self.K2_GetActorLocation`)) (.z (`self.K2_GetActorLocation`)))))

(fn `RandomMesh`
  (switch `int` (`KismetMathLibrary.RandomIntegerInRange` 0 9)
    (:`0`
      (`AddComponent|NODE_AddStaticMeshComponent-10`))
    (:`1`
      (`AddComponent|NODE_AddStaticMeshComponent-11`))
    (:`2`
      (`AddComponent|NODE_AddStaticMeshComponent-12`))
    (:`3`
      (`AddComponent|NODE_AddStaticMeshComponent-13`))
    (:`4`
      (`AddComponent|NODE_AddStaticMeshComponent-14`))
    (:`5`
      (`AddComponent|NODE_AddStaticMeshComponent-15`))
    (:`6`
      (`AddComponent|NODE_AddStaticMeshComponent-16`))
    (:`7`
      (`AddComponent|NODE_AddStaticMeshComponent-17`))
    (:`8`
      (`AddComponent|NODE_AddStaticMeshComponent-18`))
    (:`9`
      (`AddComponent|NODE_AddStaticMeshComponent-19`))))

(fn `UserConstructionScript`
  (bind _asmy_game_mode (cast `/Game/Gameplay/MyGameMode` (`GameplayStatics.GetGameMode`)))
  (set `self.speed` (`/Game/Gameplay/MyGameMode.Speed` _asmy_game_mode)))